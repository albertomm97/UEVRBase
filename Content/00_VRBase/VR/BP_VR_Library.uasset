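; BP_VR_Library is a VR Blueprint library with one function that sets the headset tracking level for seated or standing play.
; It enables the HMD, then selects Eye tracking origin for seated or Floor for standing and room-scale.
; It offsets the VR camera origin's height by the PlayerStart counter Z, adding a seated adjustment when seated.
; Both branches print the same "Seated Tracking Level" message, even standing.
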(fn `Set HMDTracking Level`
  (params (isSeated :type Boolean) (ZSeatedAdjustment :type "Float (double-precision)" :default 112.0) (PlayerStartCounterZ :type "Float (double-precision)" :default -96.870003) (VRCameraOrigin :type "SceneComponent Object Reference (by ref)"))
  (`HeadMountedDisplayFunctionLibrary.EnableHMD` true)
  (if (`local.isSeated`)
    ;[1 1 1] Seated
    (`HeadMountedDisplayFunctionLibrary.SetTrackingOrigin` "Eye")
    (`SceneComponent.K2_SetRelativeLocation` (`local.VRCameraOrigin`) (`KismetMathLibrary.MakeVector` 0.0 0.0 (+ (`local.ZSeatedAdjustment`) (`local.PlayerStartCounterZ`))) false false)
    (`KismetSystemLibrary.PrintString` null "Seated Tracking Level")
    (else
      ;[1 1 1] Standing / RoomScale
      (`HeadMountedDisplayFunctionLibrary.SetTrackingOrigin` "Floor")
      (`SceneComponent.K2_SetRelativeLocation` (`local.VRCameraOrigin`) (`KismetMathLibrary.MakeVector` 0.0 0.0 (`local.PlayerStartCounterZ`)) false false)
      (`KismetSystemLibrary.PrintString` null "Seated Tracking Level"))))